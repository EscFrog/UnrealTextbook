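; BP_TestActor is a test actor that exercises a loop, a custom function and debug printing.
; On BeginPlay it loops ten times, incrementing Number1 through its own Add function and printing each value to the screen.
; An unconnected branch, which never runs, would print in Korean whether Number1 is a two-digit number.
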(event EventBeginPlay
  (for _index (range 0 9)
    (bind _result (CallFunction|Add (Variables|Editable|GetNumber1) 1))
    (bind _output_get (Variables|Editable|SetNumber1 _result))
    (Development|PrintString (Utilities|String|ToString(Integer) _output_get) true true "(R=0.000000,G=0.660000,B=1.000000,A=1.000000)" 5.0)))

(event Collision|EventActorBeginOverlap
  (params (OtherActor :type Actor%20Object%20Reference)))

(event EventTick
  (params (DeltaSeconds :type Float%20%28single-precision%29)))

(fn ConstructionScript)

(fn Add
  (params (Num1 :type Integer) (Num2 :type Integer))
  (return (+ Num1 Num2)))